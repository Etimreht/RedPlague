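; Nails trap that periodically damages characters overlapping its sphere and wears itself out as it does.
; A Delay-driven loop from BeginPlay hits each overlapping BaseRed or ThirdPersonCharacter every cooldown, lowering the trap's Health per hit.
; BaseRed targets with default SpeedDilation also get CustomTimeDilation set to the slow rate, with no restore here.
; Tick destroys the actor once IsDead is true.
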(event EventBeginPlay
  (bind _damage (Variables|Default|GetDamage))
  (|CallParentFunction)
  (Utilities|FlowControl|Delay (Variables|Default|GetDamageCooldown) :!label _label)
  (for _array_element (Collision|GetOverlappingActors (Variables|Default|GetSphere) "/Script/Engine.Character" :!class /Script/Engine.PrimitiveComponent)
    (bind _asbase_red (Utilities|Casting|CastToBaseRed _array_element)
      (:then
        (Default|Hit _asbase_red _damage)
        (Development|PrintString (Utilities|String|ToString(Boolean) (!= (Variables|/Game/AI/Enemies/BaseRed.BaseRed_C|GetSpeedDilation _asbase_red) (.SpeedDilation (Utilities|GetClassDefaults (Utilities|GetClass _asbase_red))))))
        (if (!= (Variables|/Game/AI/Enemies/BaseRed.BaseRed_C|GetSpeedDilation _asbase_red) (.SpeedDilation (Utilities|GetClassDefaults (Utilities|GetClass _asbase_red))))
          _
          (else
            (Variables|/Script/Engine.Actor|SetCustomTimeDilation _asbase_red (Variables|Default|GetSlowRate)))))
      (:CastFailed
        (bind _asthird_person_character (Utilities|Casting|CastToThirdPersonCharacter _array_element))
        (Default|Hit _asthird_person_character _damage)))
    (Variables|Default|SetHealth (- (Variables|Default|GetHealth) (Variables|Default|GetDegradeRate)))
    (goto _label))
  (goto _label))

(event Collision|EventActorBeginOverlap
  (params (OtherActor :type Actor%20Object%20Reference))
  (|CallParentFunction OtherActor) ; This node is disabled and will not be called.\nDrag off pins to build functionality.
)

(event EventTick
  (params (DeltaSeconds :type Float%20%28single-precision%29))
  (|CallParentFunction DeltaSeconds)
  (if (Variables|Default|GetIsDead)
    (Actor|DestroyActor)))

(fn ConstructionScript
  (|CallParentFunction))