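; Flip-board trap that, while Active, damages and launches BaseRed actors in its box, and destroys itself once IsDead is set.
; Tick drives DoOnce-gated cycles: each hit applies radial force and costs the trap Health, as two chained timelines flip the board and return it, then re-arm it.
; A cooldown Delay on Tick also subtracts each overlapping BaseRed's Damage from Health.
; Active and IsDead are only read here.
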(event EventBeginPlay
  (|CallParentFunction) ; This node is disabled and will not be called.\nDrag off pins to build functionality.
)

(event Collision|EventActorBeginOverlap
  (params (OtherActor :type Actor%20Object%20Reference))
  (|CallParentFunction OtherActor) ; This node is disabled and will not be called.\nDrag off pins to build functionality.
)

(event EventTick
  (params (DeltaSeconds :type Float%20%28single-precision%29))
  (bind _staticmesh2 (Variables|Default|GetStaticMesh2))
  (|CallParentFunction DeltaSeconds)
  (if (Variables|Default|GetIsDead)
    (Actor|DestroyActor)
    (elif (Variables|Default|GetActive)
      (Utilities|FlowControl|Sequence
        (:then_0
          (Utilities|FlowControl|Sequence
            (:then_0
              (Utilities|FlowControl|DoOnce false :!label _label
                (:Completed
                  (for _array_element (Collision|GetOverlappingActors (Variables|Default|GetBox1) "/Game/AI/Enemies/BaseRed.BaseRed_C" :!class /Script/Engine.PrimitiveComponent)
                    (bind _asbase_red (Utilities|Casting|CastToBaseRed _array_element))
                    (Default|Hit _asbase_red (Variables|Default|GetDamage))
                    (Physics|AddRadialForce (Variables|/Script/Engine.Character|GetMesh _asbase_red) (Transformation|GetWorldLocation (Variables|Default|GetStaticMesh)) 2e+03 1e+04 "RIF_Linear" false))
                  (Variables|Default|SetHealth (- (Variables|Default|GetHealth) 2e+01)))))
            (:then_1
              (Utilities|FlowControl|DoOnce false :!label _label_2
                (:Completed
                  (bind _newtrack_0 (Timeline|Timeline_0 PlayFromStart)
                    (:Update
                      (Transformation|SetRelativeRotation _staticmesh2 (Math|Rotator|Lerp(Rotator) "90.000000, 0, 0" "0, 0, 0" _newtrack_0) false false))
                    (:Finished
                      (goto _label_3 Reset))))))))
        (:then_1
          (Utilities|FlowControl|Delay (Variables|Default|GetDamageCooldown))
          (for _array_element_2 (Collision|GetOverlappingActors (Variables|Default|GetBox1) "/Game/AI/Enemies/BaseRed.BaseRed_C" :!class /Script/Engine.PrimitiveComponent)
            (bind _asbase_red_2 (Utilities|Casting|CastToBaseRed _array_element_2))
            (Variables|Default|SetHealth (- (Variables|Default|GetHealth) (Variables|/Game/AI/Enemies/BaseRed.BaseRed_C|GetDamage _asbase_red_2))))))
      (else
        (Utilities|FlowControl|DoOnce false :!label _label_3
          (:Completed
            (bind _newtrack_0_2 (Timeline|Timeline_1 PlayFromStart)
              (:Update
                (Transformation|SetRelativeRotation _staticmesh2 (Math|Rotator|Lerp(Rotator) "0, 0, 0" "90.000000, 0, 0" _newtrack_0_2) false false))
              (:Finished
                (Utilities|FlowControl|Sequence
                  (:then_0
                    (goto _label_2 Reset))
                  (:then_1
                    (goto _label Reset)))))))))))

(fn ConstructionScript
  (|CallParentFunction))