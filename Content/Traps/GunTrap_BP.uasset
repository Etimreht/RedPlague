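; Gun trap that, while TrapActive is set, fires bursts of rifle bullets from its Arrow component.
; Tick uses a DoOnce to open a timed Firing window, then clears TrapActive and deducts Health.
; While Firing, every frame spawns a projectile, plays a shot sound and makes noise attributed to PlayerOwner.
; The DoOnce re-arms after DamageCooldown or whenever the trap is inactive.
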(event EventBeginPlay
  (|CallParentFunction) ; This node is disabled and will not be called.\nDrag off pins to build functionality.
)

(event Collision|EventActorBeginOverlap
  (params (OtherActor :type Actor%20Object%20Reference))
  (|CallParentFunction OtherActor) ; This node is disabled and will not be called.\nDrag off pins to build functionality.
)

(event EventTick
  (params (DeltaSeconds :type Float%20%28single-precision%29))
  (bind _arrow (Variables|Default|GetArrow))
  (bind _returnvalue (Transformation|GetWorldLocation _arrow))
  (|CallParentFunction DeltaSeconds)
  (if (Variables|Default|GetTrapActive)
    (Utilities|FlowControl|Sequence
      (:then_0
        (Utilities|FlowControl|DoOnce false :!label _label
          (:Completed
            (Variables|Default|SetFiring true)
            (Utilities|FlowControl|Delay (Variables|Default|GetFireDuration))
            (Variables|Default|SetFiring false)
            (Variables|Default|SetTrapActive false)
            (Variables|Default|SetHealth (- (Variables|Default|GetHealth) 25.0)))))
      (:then_1
        (Utilities|FlowControl|Delay (Variables|Default|GetDamageCooldown))
        (goto _label Reset))
      (:then_2
        (if (Variables|Default|GetFiring)
          (Audio|PlaySoundatLocation "/Game/SFX/RifleShot.RifleShot" _returnvalue "0, 0, 0" 1.0 1.0 0.0 "/Game/SFX/GunshotAttenuation.GunshotAttenuation" 0 0)
          (Class|Actor|MakeNoise 1.0 (Variables|Default|GetPlayerOwner) _returnvalue 2e+03 "None")
          (Game|SpawnActorfromClass "/Game/Weapons/Projectiles/Projectile_RifleBullet.Projectile_RifleBullet_C" (Transformation|GetWorldTransform _arrow) "Undefined" 0 0 0))))
    (else
      (goto _label Reset))))

(fn ConstructionScript
  (|CallParentFunction))