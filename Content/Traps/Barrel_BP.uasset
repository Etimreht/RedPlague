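; Explosive barrel trap that blows up after being shot.
; A projectile hit on the cylinder sets Health to zero.
; Tick polls IsDead, which is not set in this graph, and starts a two-second Delay once it is true.
; It then spawns a Projectile_Grenade at the barrel's location using the ExplosiveRadius sphere size, calls Explode on it and destroys the barrel.
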(event OnComponentHit(Cylinder)
  (params (HitComponent :type Primitive%20Component%20Object%20Reference) (OtherActor :type Actor%20Object%20Reference) (OtherComp :type Primitive%20Component%20Object%20Reference) (NormalImpulse :type Vector :default "0, 0, 0") (Hit :type Hit%20Result%20Structure%20%28by%20ref%29))
  (Utilities|Casting|CastToMaster_Projectile OtherActor)
  (Variables|Default|SetHealth 0.0))

(event EventBeginPlay
  (|CallParentFunction))

(event Collision|EventActorBeginOverlap
  (params (OtherActor :type Actor%20Object%20Reference))
  (|CallParentFunction OtherActor) ; This node is disabled and will not be called.\nDrag off pins to build functionality.
)

(event EventTick
  (params (DeltaSeconds :type Float%20%28single-precision%29))
  (|CallParentFunction DeltaSeconds)
  (if (Variables|Default|GetIsDead)
    (Utilities|FlowControl|Delay 2.0)
    (bind _returnvalue (Game|SpawnActorfromClass "/Game/Weapons/Projectiles/Projectile_Grenade.Projectile_Grenade_C" (Math|Conversions|ToTransform(Vector) (Transformation|GetActorLocation)) "Undefined" 0 0.0 (Variables|/Script/Engine.SphereComponent|GetSphereRadius (Variables|Default|GetExplosiveRadius)) 0 0))
    (Default|Explode _returnvalue)
    (Actor|DestroyActor)))

(fn ConstructionScript
  (|CallParentFunction))