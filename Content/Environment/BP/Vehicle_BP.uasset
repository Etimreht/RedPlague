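; Vehicle_BP is an environment vehicle prop that spawns a random item pickup when play begins.
; The construction script applies the Mesh variable to the static mesh component, so the prop's look comes from that variable.
; On BeginPlay it picks a random row name from the ItemsIndex data table and spawns an Item_Pickup with that index at the Scene component's world transform.
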(event EventBeginPlay
  (bind _outrownames (DataTable|GetDataTableRowNames "/Game/items/ItemsIndex.ItemsIndex"))
  (Game|SpawnActorfromClass "/Game/items/Item_Pickup.Item_Pickup_C" (Transformation|GetWorldTransform (Variables|Default|GetScene)) "Undefined" 0 (Utilities|Array|Get(acopy) _outrownames (Math|Random|RandomIntegerinRange 0 (- (Utilities|Array|Length _outrownames) 1))) 0.0 0))

(event Collision|EventActorBeginOverlap
  (params (OtherActor :type Actor%20Object%20Reference)))

(event EventTick
  (params (DeltaSeconds :type Float%20%28single-precision%29)))

(fn ConstructionScript
  (Components|StaticMesh|SetStaticMesh (Variables|Default|GetStaticMesh) (Variables|Default|GetMesh)))