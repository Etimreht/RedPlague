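; Blockade actor that the player clears by spending Respect, with a Cost deducted from the ThirdPersonCharacter.
; On collider overlap it polls HasPressedF through a zero-length retriggerable delay loop, then destroys itself if Respect covers Cost, otherwise prints a refusal.
; End overlap clears CollisionDetected, but the loop never reads that flag, so leaving the collider does not stop the polling.
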(event OnComponentBeginOverlap(collider)
  (params (OverlappedComponent :type Primitive%20Component%20Object%20Reference) (OtherActor :type Actor%20Object%20Reference) (OtherComp :type Primitive%20Component%20Object%20Reference) (OtherBodyIndex :type Integer) (bFromSweep :type Boolean) (SweepResult :type Hit%20Result%20Structure%20%28by%20ref%29))
  (bind _asthird_person_character (Utilities|Casting|CastToThirdPersonCharacter OtherActor))
  (bind _cost (Variables|Default|GetCost))
  (Variables|Default|SetCollisionDetected true)
  (if (Variables|/Game/ThirdPersonBP/Blueprints/ThirdPersonCharacter.ThirdPersonCharacter_C|GetHasPressedF _asthird_person_character) :!label _label
    (if (>= (Variables|/Game/ThirdPersonBP/Blueprints/ThirdPersonCharacter.ThirdPersonCharacter_C|GetRespect _asthird_person_character) _cost)
      (Actor|DestroyActor)
      (Variables|/Game/ThirdPersonBP/Blueprints/ThirdPersonCharacter.ThirdPersonCharacter_C|SetRespect _asthird_person_character (- (Variables|/Game/ThirdPersonBP/Blueprints/ThirdPersonCharacter.ThirdPersonCharacter_C|GetRespect _asthird_person_character) _cost))
      (else
        (Development|PrintString "You don't have enough respect to clear this.")))
    (else
      (Utilities|FlowControl|RetriggerableDelay 0.0)
      (goto _label))))

(event OnComponentEndOverlap(collider)
  (params (OverlappedComponent :type Primitive%20Component%20Object%20Reference) (OtherActor :type Actor%20Object%20Reference) (OtherComp :type Primitive%20Component%20Object%20Reference) (OtherBodyIndex :type Integer))
  (Utilities|Casting|CastToThirdPersonCharacter OtherActor)
  (Variables|Default|SetCollisionDetected false))

(fn ConstructionScript)